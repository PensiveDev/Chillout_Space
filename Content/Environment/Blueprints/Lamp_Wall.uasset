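; Wall lamp Blueprint whose light switches on and off with the DebugKey input action.
; BeginPlay enables input from the first player controller and applies the initial On state; each press flips that state and reapplies it.
; The On state drives point light visibility, swaps the lantern's bulb glass between glowing and plain materials, and disables the mesh's shadow casting while lit.
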(event EventBeginPlay
  (bind _pointlight (Variables|Default|GetPointLight))
  (bind _lanternv1 (Variables|Default|GetLanternV1))
  (bind _on_ (Variables|Default|GetOn?))
  (bind _lanternv1_2 (Variables|Default|GetLanternV1))
  (bind _returnvalue (not _on_))
  (Input|EnableInput (Game|GetPlayerController 0))
  (if (Variables|Default|GetOn?)
    (Rendering|SetVisibility _pointlight true true)
    (Rendering|Material|SetMaterialbyName _lanternv1_2 "BulbGlassPBS" "/Game/Environment/Static/Textures+Materials/Lantern/Materials/BulbGlassPBS_Glowing.BulbGlassPBS_Glowing")
    (Rendering|SetCastShadow _lanternv1 _returnvalue)
    (else
      (Rendering|SetVisibility _pointlight false true)
      (Rendering|Material|SetMaterialbyName _lanternv1_2 "BulbGlassPBS" "/Game/Environment/Static/Textures+Materials/Lantern/Materials/BulbGlassPBS.BulbGlassPBS")
      (Rendering|SetCastShadow _lanternv1 _returnvalue))))

(event Input|ActionEvents|InputActionDebugKey
  (params (Key :type Key%20Structure))
  (bind _pointlight (Variables|Default|GetPointLight))
  (bind _lanternv1 (Variables|Default|GetLanternV1))
  (bind _lanternv1_2 (Variables|Default|GetLanternV1))
  (:Pressed
    (if (Variables|Default|GetOn?)
      (Variables|Default|SetOn? false)
      (else
        (Variables|Default|SetOn? true)))
    (if (Variables|Default|GetOn?)
      (Rendering|SetVisibility _pointlight true true)
      (Rendering|Material|SetMaterialbyName _lanternv1_2 "BulbGlassPBS" "/Game/Environment/Static/Textures+Materials/Lantern/Materials/BulbGlassPBS_Glowing.BulbGlassPBS_Glowing")
      (Rendering|SetCastShadow _lanternv1 (not (Variables|Default|GetOn?)))
      (else
        (Rendering|SetVisibility _pointlight false true)
        (Rendering|Material|SetMaterialbyName _lanternv1_2 "BulbGlassPBS" "/Game/Environment/Static/Textures+Materials/Lantern/Materials/BulbGlassPBS.BulbGlassPBS")
        (Rendering|SetCastShadow _lanternv1 (not (Variables|Default|GetOn?)))))))

(fn ConstructionScript)