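; Cabin door Blueprint that swings open when any actor enters its trigger and shuts when an overlap ends.
; The actor's position in the door's local X axis picks a positive or negative 90-degree yaw, so the door opens away from it.
; Separate open and close timelines stop each other and lerp the mesh from its current relative rotation, easing smoothly through interruptions.
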(event OnComponentBeginOverlap(Trigger)
  (params (OverlappedComponent :type Primitive%20Component%20Object%20Reference) (OtherActor :type Actor%20Object%20Reference) (OtherComp :type Primitive%20Component%20Object%20Reference) (OtherBodyIndex :type Integer) (bFromSweep :type Boolean) (SweepResult :type Hit%20Result%20Structure%20%28by%20ref%29))
  (bind _logcabin_door_low (Variables|Default|GetLogCabin_Door_low))
  (Audio|Components|Audio|Stop (Variables|Default|GetSwing%20Closed))
  (Variables|Default|SetOpenDirection (> (.X (Math|Vector|BreakVector (Math|Vector|UnrotateVector (- (Transformation|GetActorLocation) (Transformation|GetActorLocation OtherActor)) (Transformation|GetActorRotation)))) 0.0))
  (bind _rotation (Timeline|Swing%20Open PlayFromStart)
    (:Update
      (Transformation|SetRelativeRotation _logcabin_door_low (Math|Rotator|Lerp(Rotator) (Variables|/Script/Engine.SceneComponent|GetRelativeRotation _logcabin_door_low) (Math|Rotator|MakeRotator 0.0 0.0 (Math|Float|SelectFloat 9e+01 -9e+01 (Variables|Default|GetOpenDirection))) _rotation true) false false))))

(event OnComponentEndOverlap(Trigger)
  (params (OverlappedComponent :type Primitive%20Component%20Object%20Reference) (OtherActor :type Actor%20Object%20Reference) (OtherComp :type Primitive%20Component%20Object%20Reference) (OtherBodyIndex :type Integer))
  (bind _logcabin_door_low (Variables|Default|GetLogCabin_Door_low))
  (Audio|Components|Audio|Stop (Variables|Default|GetSwing%20Open))
  (bind _newtrack_0 (Timeline|Swing%20Closed PlayFromStart)
    (:Update
      (Transformation|SetRelativeRotation _logcabin_door_low (Math|Rotator|Lerp(Rotator) (Variables|/Script/Engine.SceneComponent|GetRelativeRotation _logcabin_door_low) "0, 0, 0" _newtrack_0) false false))))

(fn ConstructionScript)