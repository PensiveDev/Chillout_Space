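; Fireplace Blueprint that toggles its fire light on and off with a debug key.
; It enables player input at BeginPlay and applies the initial On state.
; Each key press flips On, then sets the point light's visibility and makes the static mesh cast shadows only while the light is off.
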(event EventBeginPlay
  (bind _on_ (Variables|Default|GetOn?))
  (bind _returnvalue (not _on_))
  (Input|EnableInput (Game|GetPlayerController 0))
  (if (Variables|Default|GetOn?)
    (Rendering|SetVisibility (Variables|Default|GetPointLight) true true)
    (Rendering|SetCastShadow (Variables|Default|GetStaticMeshComponent0) _returnvalue)
    (else
      (Rendering|SetVisibility (Variables|Default|GetPointLight) false true)
      (Rendering|SetCastShadow (Variables|Default|GetStaticMeshComponent0) _returnvalue))))

(event EventTick
  (params (DeltaSeconds :type Float%20%28single-precision%29)))

(event Input|ActionEvents|InputActionDebugKey
  (params (Key :type Key%20Structure))
  (:Pressed
    (if (Variables|Default|GetOn?)
      (Variables|Default|SetOn? false)
      (else
        (Variables|Default|SetOn? true)))
    (if (Variables|Default|GetOn?)
      (Rendering|SetVisibility (Variables|Default|GetPointLight) true true)
      (Rendering|SetCastShadow (Variables|Default|GetStaticMeshComponent0) (not (Variables|Default|GetOn?)))
      (else
        (Rendering|SetVisibility (Variables|Default|GetPointLight) false true)
        (Rendering|SetCastShadow (Variables|Default|GetStaticMeshComponent0) (not (Variables|Default|GetOn?)))))))

(fn ConstructionScript)