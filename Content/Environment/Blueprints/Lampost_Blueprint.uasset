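; Lamppost actor Blueprint whose light can be switched on and off with a debug key.
; BeginPlay enables input from player 0, so the DebugKey action reaches the actor.
; Each press flips the On flag and sets the PointLight visibility to match, propagating to its children.
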(event EventBeginPlay
  (Input|EnableInput (Game|GetPlayerController 0)))

(event Input|ActionEvents|InputActionDebugKey
  (params (Key :type Key%20Structure))
  (:Pressed
    (if (Variables|Default|GetOn?)
      (Variables|Default|SetOn? false)
      (else
        (Variables|Default|SetOn? true)))
    (if (Variables|Default|GetOn?)
      (Rendering|SetVisibility (Variables|Default|GetPointLight) true true)
      (else
        (Rendering|SetVisibility (Variables|Default|GetPointLight) false true)))))

(fn ConstructionScript)