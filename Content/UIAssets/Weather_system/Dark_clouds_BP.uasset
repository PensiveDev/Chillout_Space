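; Dark clouds weather actor that darkens the sky into an overcast look when play begins.
; If its Sky reference is valid, a timeline blends the sky material's zenith, horizon and cloud colors toward grey while raising cloud opacity.
; The same timeline alpha dims the referenced light's color to a dark, slightly warm tone.
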(event EventBeginPlay
  (bind _sky (Variables|Default|GetSky))
  (bind _sky_material (Variables|/Engine/EngineSky/BP_Sky_Sphere.BP_Sky_Sphere_C|GetSky%20material _sky))
  (if (Utilities|IsValid (Variables|Default|GetSky))
    (bind _newtrack_0 (Timeline|Timeline_0 Play)
      (:Update
        (Rendering|Material|SetVectorParameterValue _sky_material "Zenth Color" (Math|Color|Lerp(LinearColor) "(R=0.084028,G=0.107842,B=0.166667,A=1.000000)" "(R=0.208333,G=0.208333,B=0.208333,A=1.000000)" _newtrack_0) :!class /Script/Engine.MaterialInstanceDynamic)
        (Rendering|Material|SetVectorParameterValue _sky_material "Horizon Color" (Math|Color|Lerp(LinearColor) "(R=0.104882,G=0.124038,B=0.195833,A=1.000000)" "(R=0.125000,G=0.125000,B=0.125000,A=1.000000)" _newtrack_0) :!class /Script/Engine.MaterialInstanceDynamic)
        (Rendering|Material|SetVectorParameterValue _sky_material "Cloud Color" (Math|Color|Lerp(LinearColor) "(R=0.260299,G=0.279535,B=0.304167,A=1.000000)" "(R=0.104167,G=0.104167,B=0.104167,A=1.000000)" _newtrack_0) :!class /Script/Engine.MaterialInstanceDynamic)
        (Rendering|Material|SetScalarParameterValue _sky_material "Cloud Opacity" (Math|Float|Lerp 1.2 9.0 _newtrack_0) :!class /Script/Engine.MaterialInstanceDynamic)
        (Rendering|Components|Light|SetLightColor (Variables|/Script/Engine.Light|GetLightComponent (Variables|Default|GetLight)) (Math|Color|Lerp(LinearColor) "(R=0.337500,G=0.337500,B=0.337500,A=1.000000)" "(R=0.087500,G=0.065712,B=0.058672,A=1.000000)" _newtrack_0) true)))))

(event Collision|EventActorBeginOverlap
  (params (OtherActor :type Actor%20Object%20Reference)))

(event EventTick
  (params (DeltaSeconds :type Float%20%28single-precision%29)))

(fn ConstructionScript)