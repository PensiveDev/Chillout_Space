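; Weather system lightning actor that makes a light component flash at random intervals.
; The construction script applies the configured colour, default visibility and brightness to the light.
; From BeginPlay, a random delay starts the Lightflash timeline, whose intensity curve is multiplied by a fresh random brightness on every update for flicker.
; A fixed delay off the timeline's update then loops back to the random wait.
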(event Collision|EventActorBeginOverlap
  (params (OtherActor :type Actor%20Object%20Reference)))

(event EventTick
  (params (DeltaSeconds :type Float%20%28single-precision%29)))

(event EventBeginPlay
  (Utilities|FlowControl|Delay (Math|Random|RandomFloatinRange (Variables|Lightning|GetMin%20light%20delay) (Variables|Lightning|GetMax%20light%20delay)) :!label _label)
  (bind _intensity (Timeline|Lightflash PlayFromStart)
    (:Update
      (Rendering|Components|Light|SetIntensity (Variables|Default|GetLightning) (* _intensity (Math|Random|RandomFloatinRange (Variables|Lightning|GetMin%20Brighness) (Variables|Lightning|GetMaxBrightness))))
      (Utilities|FlowControl|Delay 6.0)
      (goto _label))))

(fn ConstructionScript
  (bind _lightning (Variables|Default|GetLightning))
  (Rendering|Components|Light|SetLightColor _lightning (Variables|Lightning|Getlight%20colour) false)
  (Rendering|SetVisibility _lightning (Variables|Lightning|Getset%20default%20enable) false)
  (Rendering|Components|Light|SetIntensity _lightning (Variables|Lightning|Getbrightness)))