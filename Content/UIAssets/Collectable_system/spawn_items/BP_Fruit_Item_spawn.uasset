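; BP_Fruit_Item_spawn is a spawn point that places a random item, fruit by its name, at its own transform.
; On BeginPlay it picks a class from Itemstospawn, spawns it with itself as owner and tracks it as Currentitem.
; A Respawn event clears that reference, waits Respawndelay, then tries again, skipping the spawn if a valid item is already tracked.
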(event EventBeginPlay
  (CallFunction|Trytospawn))

(event EventRespawn
  (Variables|Default|Setcurrentitem 0)
  (Utilities|FlowControl|Delay (Variables|Default|Getrespawndelay))
  (CallFunction|Trytospawn))

(fn ConstructionScript)

(fn Trytospawn
  (Utilities|IsValid (Variables|Default|Getcurrentitem)
    (:Is%20Valid
      (Development|PrintString "item already here"))
    (:Is%20Not%20Valid
      (CallFunction|Spawn))))

(fn Spawn
  (bind _returnvalue (Game|SpawnActorfromClass (Utilities|Array|Get(acopy) (Variables|Default|Getitemstospawn) (Math|Random|RandomIntegerinRange 0 (- (Utilities|Array|Length (Variables|Default|Getitemstospawn)) 1))) (Math|Transform|MakeTransform (Transformation|GetActorLocation) (Transformation|GetActorRotation) (Transformation|GetActorScale3D)) "AdjustIfPossibleButAlwaysSpawn" self 0))
  (Variables|Default|Setcurrentitem _returnvalue))