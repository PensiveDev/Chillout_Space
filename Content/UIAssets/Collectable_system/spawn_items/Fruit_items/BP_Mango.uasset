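; BP_Mango is a collectable mango pickup that stores itself in the player's inventory slots.
; When anything overlaps its Box, it casts player 0's pawn to FirstPersonCharacter without checking which actor overlapped.
; A nested branch chain writes item ID 9 into the first empty slot of twelve, then destroys the actor.
; If every slot is occupied, it prints "All Found" and stays in the world.
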(event OnComponentBeginOverlap(Box)
  (params (OverlappedComponent :type Primitive%20Component%20Object%20Reference) (OtherActor :type Actor%20Object%20Reference) (OtherComp :type Primitive%20Component%20Object%20Reference) (OtherBodyIndex :type Integer) (bFromSweep :type Boolean) (SweepResult :type Hit%20Result%20Structure%20%28by%20ref%29))
  (bind _asfirst_person_character (Utilities|Casting|CastToFirstPersonCharacter (Game|GetPlayerCharacter 0)))
  (if (== (Variables|/Game/FirstPersonBP/Blueprints/FirstPersonCharacter.FirstPersonCharacter_C|GetSlot1 _asfirst_person_character) 0)
    (Variables|/Game/FirstPersonBP/Blueprints/FirstPersonCharacter.FirstPersonCharacter_C|SetSlot1 _asfirst_person_character 9)
    (Actor|DestroyActor :!label _label)
    (elif (== (Variables|/Game/FirstPersonBP/Blueprints/FirstPersonCharacter.FirstPersonCharacter_C|GetSlot2 _asfirst_person_character) 0)
      (Variables|/Game/FirstPersonBP/Blueprints/FirstPersonCharacter.FirstPersonCharacter_C|SetSlot2 _asfirst_person_character 9)
      (goto _label)
      (elif (== (Variables|/Game/FirstPersonBP/Blueprints/FirstPersonCharacter.FirstPersonCharacter_C|Getslot3 _asfirst_person_character) 0)
        (Variables|/Game/FirstPersonBP/Blueprints/FirstPersonCharacter.FirstPersonCharacter_C|Setslot3 _asfirst_person_character 9)
        (goto _label)
        (elif (== (Variables|/Game/FirstPersonBP/Blueprints/FirstPersonCharacter.FirstPersonCharacter_C|Getslot4 _asfirst_person_character) 0)
          (Variables|/Game/FirstPersonBP/Blueprints/FirstPersonCharacter.FirstPersonCharacter_C|Setslot4 _asfirst_person_character 9)
          (goto _label)
          (elif (== (Variables|/Game/FirstPersonBP/Blueprints/FirstPersonCharacter.FirstPersonCharacter_C|Getslot5 _asfirst_person_character) 0)
            (Variables|/Game/FirstPersonBP/Blueprints/FirstPersonCharacter.FirstPersonCharacter_C|Setslot5 _asfirst_person_character 9)
            (goto _label)
            (elif (== (Variables|/Game/FirstPersonBP/Blueprints/FirstPersonCharacter.FirstPersonCharacter_C|Getslot6 _asfirst_person_character) 0)
              (Variables|/Game/FirstPersonBP/Blueprints/FirstPersonCharacter.FirstPersonCharacter_C|Setslot6 _asfirst_person_character 9)
              (goto _label)
              (elif (== (Variables|/Game/FirstPersonBP/Blueprints/FirstPersonCharacter.FirstPersonCharacter_C|Getslot7 _asfirst_person_character) 0)
                (Variables|/Game/FirstPersonBP/Blueprints/FirstPersonCharacter.FirstPersonCharacter_C|Setslot7 _asfirst_person_character 9)
                (goto _label)
                (elif (== (Variables|/Game/FirstPersonBP/Blueprints/FirstPersonCharacter.FirstPersonCharacter_C|Getslot8 _asfirst_person_character) 0)
                  (Variables|/Game/FirstPersonBP/Blueprints/FirstPersonCharacter.FirstPersonCharacter_C|Setslot8 _asfirst_person_character 9)
                  (goto _label)
                  (elif (== (Variables|/Game/FirstPersonBP/Blueprints/FirstPersonCharacter.FirstPersonCharacter_C|Getslot9 _asfirst_person_character) 0)
                    (Variables|/Game/FirstPersonBP/Blueprints/FirstPersonCharacter.FirstPersonCharacter_C|Setslot9 _asfirst_person_character 9)
                    (goto _label)
                    (elif (== (Variables|/Game/FirstPersonBP/Blueprints/FirstPersonCharacter.FirstPersonCharacter_C|Getslot10 _asfirst_person_character) 0)
                      (Variables|/Game/FirstPersonBP/Blueprints/FirstPersonCharacter.FirstPersonCharacter_C|Setslot10 _asfirst_person_character 9)
                      (goto _label)
                      (elif (== (Variables|/Game/FirstPersonBP/Blueprints/FirstPersonCharacter.FirstPersonCharacter_C|Getslot11 _asfirst_person_character) 0)
                        (Variables|/Game/FirstPersonBP/Blueprints/FirstPersonCharacter.FirstPersonCharacter_C|Setslot11 _asfirst_person_character 9)
                        (goto _label)
                        (elif (== (Variables|/Game/FirstPersonBP/Blueprints/FirstPersonCharacter.FirstPersonCharacter_C|Getslot12 _asfirst_person_character) 0)
                          (Variables|/Game/FirstPersonBP/Blueprints/FirstPersonCharacter.FirstPersonCharacter_C|Setslot12 _asfirst_person_character 9)
                          (goto _label)
                          (else
                            (Development|PrintString "All Found")))))))))))))))

(fn ConstructionScript
  (|CallParentFunction))