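; Fish character that swims toward a Destination, using either the angelfish or default swimming fish mesh and anim blueprint, chosen by IsAngel at construction.
; MoveToDestination plays the MoveUntil timeline, which blends capsule rotation toward the target while adding forward movement input.
; Outside the timeline's turning phase, it stops when a line trace to the ProximitySensor hits or the fish is near the Destination.
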(event Custom|MoveToDestination
  (bind _returnvalue (Transformation|GetActorLocation))
  (Utilities|FlowControl|Sequence
    (:then_0
      (Variables|Default|SetTurning? false :!label _label)
      (bind _rotation (Timeline|MoveUntil Stop)
        (:Update
          (Transformation|SetWorldRotation (Variables|Collision|GetCapsuleComponent) (Math|Rotator|Lerp(Rotator) (Transformation|GetWorldRotation (Variables|Collision|GetCapsuleComponent)) (Math|Rotator|FindLookatRotation (Transformation|GetActorLocation) (Variables|Default|GetDestination)) _rotation true) false false)
          (Pawn|Input|AddMovementInput (Transformation|GetActorForwardVector) 1.0 false)
          (bind _returnvalue_2 (Collision|LineTraceByChannel _returnvalue (Transformation|GetWorldLocation (Variables|Default|GetProximitySensor)) "TraceTypeQuery1" false 0 "None" true "(R=1.000000,G=0.000000,B=0.000000,A=1.000000)" "(R=0.000000,G=1.000000,B=0.000000,A=1.000000)" 1.0))
          (if (and (or _returnvalue_2 (Math|Vector|Equal(Vector) _returnvalue (Variables|Default|GetDestination) 5e+01)) (not (Variables|Default|GetTurning?)))
            (goto _label)))
        (:Rotating
          (Variables|Default|SetTurning? true))
        (:NotRotating
          (Variables|Default|SetTurning? false))))
    (:then_1
      (Timeline|MoveUntil PlayFromStart))))

(event EventBeginPlay)

(event Collision|EventActorBeginOverlap
  (params (OtherActor :type Actor%20Object%20Reference)))

(event EventTick
  (params (DeltaSeconds :type Float%20%28single-precision%29)))

(fn ConstructionScript
  (bind _mesh (Variables|Character|GetMesh))
  (bind _mesh_2 (Variables|Character|GetMesh))
  (if (Variables|Default|GetIsAngel?)
    (Class|SkinnedMeshComponent|SetSkeletalMesh _mesh_2 "/Game/Animals/Fish/ANGELFISH/AngelFish_Rig.AngelFish_Rig" true)
    (Components|SkeletalMesh|SetAnimInstanceClass _mesh_2 "/Game/Animals/Fish/ANGELFISH/AngelFish_Rig_Skeleton_AnimBlueprint.AngelFish_Rig_Skeleton_AnimBlueprint_C")
    (else
      (Class|SkinnedMeshComponent|SetSkeletalMesh _mesh "/Game/Animals/Fish/CLOWNFISH/Fish_Swim_Rig.Fish_Swim_Rig" true)
      (Components|SkeletalMesh|SetAnimInstanceClass _mesh "/Game/Animals/Fish/CLOWNFISH/Fish_Swim_Rig_Skeleton_AnimBlueprint.Fish_Swim_Rig_Skeleton_AnimBlueprint_C"))))